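; Game mode for a trip game played across BP_Local locations: sets up the HUD, players and match start.
; BeginPlay maps locations by index, then has location 0's spawner create pawns from the "Bots" save.
; StartGame fires after each optional pawn (2–4), so can repeat, or once if there are none.
; SetAeroporto stores the airport player and flags every location; its bot branch is empty.
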(event `self.ReceiveBeginPlay`
  ;[0.8529 1 0.666] Create
  (bind _returnvalue (`|CreateWidget` "/Game/Widgets/BP_WidgetGame.BP_WidgetGame_C"))
  (set `self.WidgetGame` _returnvalue)
  (`UserWidget.AddToViewport` _returnvalue 0)
  (bind _outactors (`GameplayStatics.GetAllActorsOfClass` "/Game/Lugares/BP_Local.BP_Local_C"))
  (for _array_element _outactors
    (`BlueprintMapLibrary.Map_Add` (`self.MapLocals`) (`/Game/Lugares/BP_Local.LocalIndex` _array_element) _array_element)
    (`KismetArrayLibrary.Array_Add` (`self.MapArray`) _array_element))
  (bind _returnvalue_2 (`GameplayStatics.LoadGameFromSlot` "Bots"))
  (bind _asbp_save_game (cast `/Game/SaveGame/BP_SaveGame` _returnvalue_2))
  (bind _asbp_local_spawm (`self.Get Spawn`))
  (`/Game/Lugares/BP_LocalSpawm.Event Create Pawn 1` _asbp_local_spawm (`/Game/SaveGame/BP_SaveGame.TextX1` _asbp_save_game))
  (`|ExecutionSequence`
    (:`then_0`
      (bind _isplayerx2 (`/Game/SaveGame/BP_SaveGame.isPlayerX2` _asbp_save_game))
      (if _isplayerx2
        (`/Game/Lugares/BP_LocalSpawm.Event Create Pawn 2` _asbp_local_spawm (`/Game/SaveGame/BP_SaveGame.TextX2` _asbp_save_game))
        (`/Game/Lugares/BP_LocalSpawm.Start Game` _asbp_local_spawm :!label _label)))
    (:`then_1`
      (bind _isplayerx3 (`/Game/SaveGame/BP_SaveGame.isPlayerX3` _asbp_save_game))
      (if _isplayerx3
        (`/Game/Lugares/BP_LocalSpawm.Event Create Pawn 3` _asbp_local_spawm (`/Game/SaveGame/BP_SaveGame.TextX3` _asbp_save_game))
        (goto _label)))
    (:`then_2`
      (bind _isplayerx4 (`/Game/SaveGame/BP_SaveGame.isPlayerX4` _asbp_save_game))
      (if _isplayerx4
        (`/Game/Lugares/BP_LocalSpawm.Event Create Pawn 4` _asbp_local_spawm (`/Game/SaveGame/BP_SaveGame.TextX4` _asbp_save_game))
        (goto _label)))
    (:`then_3`
      (if (not (or _isplayerx2 _isplayerx3 _isplayerx4))
        (goto _label)))))

(event `Event Set Aeroporto`
  (params (Player :type "/Game/GameComponents/BP_PlayerTrip Object Reference"))
  (set `self.PlayerInAeroporto` Player)
  (for _array_element (`self.MapArray`)
    ;[1 1 1] Continua
    (set `/Game/Lugares/BP_Local.isAeroporto` true _array_element)
    (if (`/Game/GameComponents/BP_PlayerTrip.isBot` Player)
      _)))

(fn `Get Spawn`
  (returns (`AsBP Local Spawm` :type "/Game/Lugares/BP_LocalSpawm Object Reference"))
  (bind _asbp_local_spawm (cast `/Game/Lugares/BP_LocalSpawm` (`BlueprintMapLibrary.Map_Find` (`self.MapLocals`)))
    (:`then`
      (return _asbp_local_spawm))
    (:`CastFailed`
      (`KismetSystemLibrary.PrintString` "DEU FALHO NA QUELE GACARA CA" true true (struct :`R` 0.350842 :`B` 1.0 :`A` 1.0)))))

(fn `Update Widget`)

(fn `UserConstructionScript`)