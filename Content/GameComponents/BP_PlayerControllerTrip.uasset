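; Player controller for a four-player, dice-based board game with money and clickable BP_Local spots.
; SetPlayer stores the players, pushes names and money to the game mode's widget, binds the dice event and shows the dice widget.
; Each dice event moves the current player by a test value rather than the two-die random helper, with turn index falling back to 2 after 3.
; Left clicks trace under the cursor to trigger BP_Local's click event.
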(event `Event Dice And Moviment`
  (bind _teste (`self.Teste`))
  (bind _indexgo (`self.IndexGo`))
  (bind _output (`|GetArrayItem` (`self.Players`) (`self.IndexGo`)))
  (`/Game/GameComponents/BP_PlayerTrip.EventSetLocalDestiny` _output _teste)
  (`/Game/GameComponents/BP_PlayerTrip.Movement` _output _teste)
  (if (== _indexgo 3)
    (set `self.IndexGo` 2)
    (set `self.Teste` 10)
    (else
      (`/Engine/EditorBlueprintResources/StandardMacros.IncrementInt` _indexgo))))

(event `Event Set Player`
  (params (Player :type "/Game/GameComponents/BP_PlayerTrip Object Reference") (Player2 :type "/Game/GameComponents/BP_PlayerTrip Object Reference") (Player3 :type "/Game/GameComponents/BP_PlayerTrip Object Reference") (Player4 :type "/Game/GameComponents/BP_PlayerTrip Object Reference"))
  (`self.SetPlayers` Player Player2 Player3 Player4
    (:`NewParam`
      (set `self.Players` (`|MakeArray` Player Player2 Player3 Player4))
      (`self.UpdateWidget`)
      (add `self.EventClickGoDice` (delegate `Event Dice And Moviment`))
      (bind _returnvalue (`|CreateWidget` "/Game/Widgets/BP_PlayDice.BP_PlayDice_C"))
      (`UserWidget.AddToViewport` _returnvalue 0))))

(event `Key|LeftMouseButton`
  (params (Key :type "Key Structure"))
  ;[1 1 1] é isso
  (:`Pressed`
    (bind _asbp_local (cast `/Game/Lugares/BP_Local` (`.HitActor` (`GameplayStatics.BreakHitResult` (`self.GetHitResultUnderCursorByChannel` "TraceTypeQuery1")))))
    (`/Game/Lugares/BP_Local.ClickEvent` _asbp_local)))

(fn `Get Randoms`
  (returns (Random1 :type Integer) (Random2 :type Integer))
  (bind _returnvalue (`self.Random`)
    (:`Go`
      (set `self.RandomAll` _returnvalue)
      (return (`self.Random1`) (`self.Random2`)))))

(fn `UpdateWidget`
  (`self.Set Widget Players` (`self.Player1`) (`self.Player2`) (`self.Player3`) (`self.Player4`)))

(fn `UserConstructionScript`)