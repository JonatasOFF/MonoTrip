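; BP_PlayerTrip is a player pawn for a dice-driven board game, tracking board position, money, owned locations and a beach level.
; Movement repeats a timeline lerp one tile at a time through the GameMode's MapLocals, using per-player slots and wrapping the index.
; The destination tile lights up during travel, then switches off and receives the pawn on arrival.
; SetNewMoney applies payments, refreshing widgets or showing a cannot-buy widget when funds are short.
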(event `Movement`
  (params (RandomMovement :type Integer))
  ;[0.7853 1 0.8178] MovimentOfPawn
  (`self.SetRandomAndLocalVectorScene` RandomMovement)
  (bind (_direction _movementforward) (`Timeline|MovementPawn` :!via `PlayFromStart`)
    (:`Update`
      (`self.SetLocalMovimentAndAnimation` _movementforward))
    (:`Finished`
      ;[1 1 1] Account
      (bind _objectlocal (`self.SetLocalPawnAndAccount`)
        (:`FInal`
          (`/Game/Lugares/BP_Local.Event Off Light` _objectlocal)
          (`/Game/Lugares/BP_Local.EuSouEsse` _objectlocal)
          ;;[1 1 1] Chegou no local
          (`/Game/Lugares/BP_Local.Call Local` _objectlocal self))
        (:`Go`
          (`self.Movement` (`self.Random Movement`)))))))

(event `self.ReceiveBeginPlay`
  ;[0.5174 1 0.7373] Set Map Locals
  (bind _asbp_game_mode_trip (cast `/Game/GameComponents/BP_GameModeTrip` (`GameplayStatics.GetGameMode`)))
  (set `self.MapLocals` (`/Game/GameComponents/BP_GameModeTrip.MapLocals` _asbp_game_mode_trip)))

(event `CreatePawn`
  (params (IndexScene :type Integer) (NamePlayer :type Text) (MaterialPlayer :type "MaterialInstance Object Reference"))
  ;[1 0.7762 0.6224] Set Scene Local
  (set `self.NamePlayer` NamePlayer)
  (set `self.IndexScene` IndexScene)
  (set `self.LocalWorld` (`SceneComponent.K2_GetComponentLocation` (`self.DefaultSceneRoot`)))
  (`PrimitiveComponent.SetMaterial` (`self.Cone`) 0 MaterialPlayer))

(event `Event Add Locals Get`
  (params (LocalGet :type "/Game/Lugares/BP_Local Object Reference"))
  (`KismetArrayLibrary.Array_Add` (`self.LocalsHave`) LocalGet))

(event `EventSetLocalDestiny`
  (params (`House Walk` :type Integer))
  (bind _returnvalue (`BlueprintMapLibrary.Map_Length` (`self.MapLocals`)))
  (bind _returnvalue_2 (+ (`self.IndexNow`) (`self.HouseWalk`)))
  ;[1 1 1] Local Go
  (set `self.HouseWalk` `House Walk`)
  (if (>= _returnvalue_2 _returnvalue)
    (set `self.IndexNow` (- _returnvalue_2 _returnvalue))
    (else
      (set `self.IndexNow` _returnvalue_2))))

(event `Event Beach add`
  (`/Engine/EditorBlueprintResources/StandardMacros.IncrementInt` (`self.LevelBeach`)))

(fn `SetNewMoney`
  (params (ValuePay :type Integer) (isSetPlay :type Boolean :default false))
  (returns (isSetMoney :type Boolean))
  (locals (Widget :type "/Game/Widgets/BP_WidgetNotBuyThis Object Reference") (isSet :type Boolean))
  (bind _returnvalue (- (`self.Money`) ValuePay))
  (if (< ValuePay 0)
    (set `self.Money` _returnvalue :!label _label)
    (bind _asbp_player_controller_trip (cast `/Game/GameComponents/BP_PlayerControllerTrip` (`GameplayStatics.GetPlayerController` 0)))
    (`/Game/GameComponents/BP_PlayerControllerTrip.SetWidgets` _asbp_player_controller_trip)
    (if isSetPlay
      (bind _foundwidgets (`WidgetBlueprintLibrary.GetAllWidgetsOfClass` "/Game/Widgets/BP_PlayDice.BP_PlayDice_C"))
      (`/Game/Widgets/BP_PlayDice.EventShowClickGo` (`|GetArrayItem` _foundwidgets)))
    (set `local.isSet` true)
    (elif (< _returnvalue 0)
      (`KismetSystemLibrary.PrintString` "Sem Dinheiro" true true (struct :`R` 1.0 :`B` 0.060073 :`A` 1.0) 50.0)
      (bind _returnvalue_2 (`|CreateWidget` "/Game/Widgets/BP_WidgetNotBuyThis.BP_WidgetNotBuyThis_C"))
      (bind _output_get (set `local.Widget` _returnvalue_2))
      (`UserWidget.AddToViewport` _output_get 0)
      (set `local.isSet` false)
      (else
        (goto _label))))
  (return (`local.isSet`)))

(fn `UserConstructionScript`)