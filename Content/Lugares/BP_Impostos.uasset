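; BP_Impostos is a tax space among the game's locations that charges a player who triggers it.
; CallLocal stores the player and calls SetNewMoney, flagged as a tax, with the tax value multiplied by the number of locations that player owns.
; It then calls GoNextRound to advance the game.
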(event `self.Call Local`
  (params (PlayerTrip :type "/Game/GameComponents/BP_PlayerTrip Object Reference"))
  (bind _output_get (set `self.Player` PlayerTrip))
  (`/Game/GameComponents/BP_PlayerTrip.SetNewMoney` _output_get (* (`self.ValueTaxImpostos`) (`KismetArrayLibrary.Array_Length` (`/Game/GameComponents/BP_PlayerTrip.LocalsHave` _output_get))) false true)
  (`/Game/FunctionsBot/BP_FunctionFromBot.Go Next Round`))

(fn `UserConstructionScript`
  (`parent.UserConstructionScript`))