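; Buyable house tile for a dice board game, with four upgrade levels priced from its board index and a compounding multiplier.
; CallLocal offers purchase or upgrade, shows the dice prompt when maxed, or charges visitors tax and offers repurchase.
; BuyHouseByLevel handles payment, cascades house visibility, applies the player's material and sets ownership; level 2's payment logic is disconnected.
; SetValueTax derives tax from property value and formats its K/M label.
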(event `self.ReceiveBeginPlay`
  (`parent.ReceiveBeginPlay`)
  (bind _output_get (`self.Set Multiply Per House And Price`))
  (`self.Set Value Of House` _output_get))

(event `self.Call Local`
  (params (PlayerTrip :type "/Game/GameComponents/BP_PlayerTrip Object Reference"))
  (bind _output_get (set `self.PlayerNow` PlayerTrip))
  (if (== null (`self.PlayerBuyToHouse`))
    ;[1 1 1] Casa ainda não comprada
    (bind _returnvalue (`|CreateWidget` "/Game/Widgets/BP_WidgetBuy.BP_WidgetBuy_C"))
    (bind _output_get_2 (set `self.WidgetBuyHouse` _returnvalue))
    (`/Game/Widgets/BP_WidgetBuy.Event Show Widget For Player` _output_get_2 self (`self.ValueHouse1`) (`self.ValueHouse2`) (`self.ValueHosue3`) (`self.ValueHouse4`) 0 false)
    (`UserWidget.AddToViewport` _output_get_2 0)
    (elif (== _output_get (`self.PlayerBuyToHouse`))
      ;[1 1 1] Casa Foi Comprada, mas é do mesmo player
      (if (== (`self.LevelHouse`) 4)
        (bind _foundwidgets (`WidgetBlueprintLibrary.GetAllWidgetsOfClass` "/Game/Widgets/BP_PlayDice.BP_PlayDice_C"))
        (`/Game/Widgets/BP_PlayDice.ShowClickGo` (`|GetArrayItem` _foundwidgets))
        (else
          (bind _returnvalue_2 (`|CreateWidget` "/Game/Widgets/BP_WidgetBuy.BP_WidgetBuy_C"))
          (bind _output_get_3 (set `self.WidgetBuyHouse` _returnvalue_2))
          (`/Game/Widgets/BP_WidgetBuy.Event Show Widget For Player` _output_get_3 self (`self.ValueHouse1`) (`self.ValueHouse2`) (`self.ValueHosue3`) (`self.ValueHouse4`) (`self.LevelHouse`) true)
          (`UserWidget.AddToViewport` _output_get_3 0)))
      (else
        ;[1 1 1] Casa já foi comprada, mas é de outro player
        (`self.SetPayment` false (`self.ValueTax`))
        (bind _returnvalue_3 (`|CreateWidget` "/Game/Widgets/BP_Repurchase.BP_Repurchase_C"))
        (`/Game/Widgets/BP_Repurchase.Event Show Widget To Repurchase` _returnvalue_3 self (`self.ValueToBuyAllHouses`) (`self.LevelHouse`))
        (`UserWidget.AddToViewport` _returnvalue_3 0)))))

(fn `BuyHouseByLevel`
  (params (LevelHouse :type Integer) (isChargeMoneyPlayer :type Boolean))
  (set `self.isChargeMoneyPlayer` isChargeMoneyPlayer)
  (bind _output_get (set `self.LevelHouse` LevelHouse))
  (switch `int` _output_get
    (:`1`
      (`self.Set Solo House 1`)
      (`self.SetHouse1`))
    (:`2`
      (`self.Set Solo House 2`)
      (`self.Set House 2`))
    (:`3`
      (`self.Set Solo House 3`
        (:`exec`
          (`self.Set House 3`))))
    (:`4`
      (`self.Set Solo House 4`)
      (`self.Set House 4`))))

(fn `SetPayment`
  (params (isSetPlay :type Boolean) (ValueGoPay :type Integer))
  (`/Game/GameComponents/BP_PlayerTrip.SetNewMoney` (`self.PlayerNow`) ValueGoPay false)
  (`/Game/GameComponents/BP_PlayerTrip.SetNewMoney` (`self.PlayerBuyToHouse`) (* ValueGoPay -1) isSetPlay))

(fn `SetRound`
  (returns (ReturnValue :type Text))
  (locals (ValueTaxShow :type "Float (double-precision)") (SetLetter :type String))
  (bind _valuetax (`self.ValueTax`))
  (set `local.ValueTaxShow` (`KismetMathLibrary.Conv_IntToDouble` _valuetax))
  (if (>= _valuetax 1000000)
    (set `local.SetLetter` "M")
    (set `local.ValueTaxShow` (/ (`local.ValueTaxShow`) 1000000.0))
    (else
      (set `local.SetLetter` "K")
      (set `local.ValueTaxShow` (/ (`local.ValueTaxShow`) 1000.0))))
  (return (`KismetTextLibrary.Conv_StringToText` (`KismetStringLibrary.Concat_StrStr` (`KismetTextLibrary.Conv_TextToString` (`KismetTextLibrary.Conv_DoubleToText` (`local.ValueTaxShow`) "HalfToEven")) (`local.SetLetter`)))))

(fn `SetValueTax`
  (bind _output_get (set `self.ValueTax` (`KismetMathLibrary.FTrunc` (/ (`KismetMathLibrary.Conv_IntToDouble` (`self.ValueToBuyAllHouses`)) (`self.Reason Tax`)))))
  (bind _returnvalue (`self.SetRound`))
  (`TextRenderComponent.K2_SetText` (`self.ValueTaxToPay`) _returnvalue)
  (`KismetSystemLibrary.PrintString` (`KismetStringLibrary.Conv_IntToString` _output_get) true true (struct :`G` 0.66 :`B` 1.0 :`A` 1.0) 90.0))

(fn `UserConstructionScript`
  (`parent.UserConstructionScript`))