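; BP_Local is a location actor for a named nation, showing its uppercase name and lighting up under the mouse cursor.
; BeginPlay enables the cursor and mouse-over events, and hovering Inside or Plane shows the PointLight.
; OnLight and OffLight set a flag that keeps the light on after hover ends, and print the nation name.
; GetSceneForPlayer maps an index to one of four PlayerStay world positions, while CallLocal is an empty stub.
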(event `Call Local`
  (params (PlayerTrip :type "/Game/GameComponents/BP_PlayerTrip Object Reference")))

(event `self.ReceiveBeginPlay`
  (bind _returnvalue (`GameplayStatics.GetPlayerController` 0))
  (`self.EnableInput` _returnvalue)
  (`TextRenderComponent.K2_SetText` (`self.TextRender`) (`KismetTextLibrary.TextToUpper` (`self.NameNation`)))
  (set `PlayerController.bShowMouseCursor` true _returnvalue)
  (set `PlayerController.bEnableMouseOverEvents` true _returnvalue))

(event `ClickEvent`
  ;[0.2118 0.9002 1] Event Detect Mouse Cursor
  (`KismetSystemLibrary.PrintString` "rola"))

(event `self.Inside.OnBeginCursorOver`
  (params (TouchedComponent :type "PrimitiveComponent Object Reference"))
  ;[0.2118 0.9002 1] Event Detect Mouse Cursor
  ;;[1 0.06069 0] Event Light Cursor
  (`SceneComponent.SetVisibility` (`self.PointLight`) true false :!label _label))

(event `self.ReceiveActorEndCursorOver`
  ;[0.2118 0.9002 1] Event Detect Mouse Cursor
  ;;[1 0.06069 0] Event Light Cursor
  (if (not (`self.isLightOnPlayerGo`)) :!label _label_2
    (`SceneComponent.SetVisibility` (`self.PointLight`) false false)))

(event `self.Plane.OnBeginCursorOver`
  (params (TouchedComponent :type "PrimitiveComponent Object Reference"))
  ;[0.2118 0.9002 1] Event Detect Mouse Cursor
  ;;[1 0.06069 0] Event Light Cursor
  (goto _label))

(event `self.Plane.OnEndCursorOver`
  (params (TouchedComponent :type "PrimitiveComponent Object Reference"))
  ;[0.2118 0.9002 1] Event Detect Mouse Cursor
  ;;[1 0.06069 0] Event Light Cursor
  (goto _label_2))

(event `Event On Light`
  ;[0.2118 0.9002 1] Event Detect Mouse Cursor
  ;;[1 0.06069 0] Event Light Cursor
  (bind _output_get (set `self.isLightOnPlayerGo` true))
  (`SceneComponent.SetVisibility` (`self.PointLight`) _output_get false)
  (`self.EuSouEsse`))

(event `Event Off Light`
  (bind _output_get (set `self.isLightOnPlayerGo` false))
  (`SceneComponent.SetVisibility` (`self.PointLight`) _output_get false)
  (`self.EuSouEsse`))

(fn `EuSouEsse`
  (`KismetSystemLibrary.PrintString` (`KismetTextLibrary.Conv_TextToString` (`self.NameNation`))))

(fn `Get Scene for Player`
  (params (IndexScene :type Integer))
  (returns (ReturnVector :type "Vector Structure"))
  (switch `int` IndexScene
    (:`1`
      (set `self.SetSceneComponentForPlayer` (`self.PlayerStay`)))
    (:`2`
      (set `self.SetSceneComponentForPlayer` (`self.PlayerStay1`)))
    (:`3`
      (set `self.SetSceneComponentForPlayer` (`self.PlayerStay2`)))
    (:`4`
      (set `self.SetSceneComponentForPlayer` (`self.PlayerStay3`))))
  (return (`SceneComponent.K2_GetComponentLocation` (`self.SetSceneComponentForPlayer`))))

(fn `UserConstructionScript`)