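; Beach property space for what appears to be a Monopoly-style board game, which players can buy or pay tax on.
; CallLocal opens BP_WidgetBeach when the beach has no owner, otherwise charges visitors other than the owner ValueTaxBeach.
; BeachBuy records the owner and reveals the Beach component in that player's sphere material.
; SetPaymanet settles the tax through both players' SetNewMoney, negating the value for the owner.
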(event `self.Call Local`
  (params (PlayerTrip :type "/Game/GameComponents/BP_PlayerTrip Object Reference"))
  (bind _output_get (set `self.PlayerNow` PlayerTrip))
  (if (== null (`self.PlayerBuyToHouse`))
    (bind _returnvalue (`|CreateWidget` "/Game/Widgets/BP_WidgetBeach.BP_WidgetBeach_C"))
    (`/Game/Widgets/BP_WidgetBeach.ShowWidgetBeach` _returnvalue (`self.PlayerNow`) self)
    (`UserWidget.AddToViewport` _returnvalue 0)
    (elif (not (== _output_get (`self.PlayerBuyToHouse`)))
      (`self.Set Paymanet` (`self.ValueTaxBeach`) true))))

(event `BeachBuy`
  (bind _beach (`self.Beach`))
  (`SceneComponent.SetVisibility` _beach true false)
  (`PrimitiveComponent.SetMaterial` _beach 0 (`PrimitiveComponent.GetMaterial` (`/Game/GameComponents/BP_PlayerTrip.Sphere` (`self.PlayerNow`)) 0))
  (set `self.PlayerBuyToHouse` (`self.PlayerNow`)))

(fn `Set Paymanet`
  (params (ValuePay :type Integer) (isSetPlay :type Boolean))
  (`/Game/GameComponents/BP_PlayerTrip.SetNewMoney` (`self.PlayerNow`) ValuePay false)
  (`/Game/GameComponents/BP_PlayerTrip.SetNewMoney` (`self.PlayerBuyToHouse`) (* ValuePay -1) isSetPlay))

(fn `UserConstructionScript`
  (`parent.UserConstructionScript`))