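; BP_LocalSpecialAmazonia is the special Amazonia location, one of the game's places (Lugares).
; Its CallLocal event stores the passed player as Player0, sets that player's IsAmazonia flag and calls GoNextRound with it.
; A leftover debug PrintString runs at the end, and the construction script only calls its parent.
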(event `/Game/Lugares/BP_Local.Call Local`
  (params (PlayerTrip :type "/Game/GameComponents/BP_PlayerTrip Object Reference"))
  (bind _output_get (set `self.Player_0` PlayerTrip))
  (set `/Game/GameComponents/BP_PlayerTrip.isAmazonia` true _output_get)
  (`/Game/FunctionsBot/BP_FunctionFromBot.Go Next Round` _output_get)
  (`KismetSystemLibrary.PrintString` "hsdffsadffds" true true (struct :`R` 1.0 :`G` 0.068094 :`A` 1.0) 50.0))

(fn `UserConstructionScript`
  (`parent.UserConstructionScript`))