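; Level spawn point actor that creates up to four BP_PlayerTrip pawns, the first as the player and the other three flagged as bots.
; On BeginPlay it enables input and calls Create on BP_GameModeTrip.
; Each CreatePawn event spawns a half-scale pawn at its own PlayerStay marker, setting index, name and material.
; StartGame passes the collected pawn array to BP_PlayerControllerTrip through EventSetPlayer.
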(event `self.ReceiveBeginPlay`
  (`parent.ReceiveBeginPlay`)
  (`self.EnableInput` (`GameplayStatics.GetPlayerController` 0))
  (bind _asbp_game_mode_trip (cast `/Game/GameComponents/BP_GameModeTrip` (`GameplayStatics.GetGameMode`)))
  (`/Game/GameComponents/BP_GameModeTrip.Create` _asbp_game_mode_trip))

(event `Event Create Pawn 1`
  (params (Name :type Text))
  (bind _returnvalue (`|SpawnActorFromClass` "/Game/GameComponents/BP_PlayerTrip.BP_PlayerTrip_C" (`KismetMathLibrary.MakeTransform` (`SceneComponent.K2_GetComponentLocation` (`self.PlayerStay`)) (struct) (0.5 0.5 0.5)) "AlwaysSpawn" "OverrideRootScale" null null))
  (`/Game/GameComponents/BP_PlayerTrip.CreatePawn` _returnvalue 1 Name (`BlueprintMapLibrary.Map_Find` (`self.Materials`) 1) false)
  (`KismetArrayLibrary.Array_Add` (`self.ArrayPlayersSpawn`) _returnvalue))

(event `Event Create Pawn 2`
  (params (Name :type Text))
  (bind _returnvalue (`|SpawnActorFromClass` "/Game/GameComponents/BP_PlayerTrip.BP_PlayerTrip_C" (`KismetMathLibrary.MakeTransform` (`SceneComponent.K2_GetComponentLocation` (`self.PlayerStay1`)) (struct) (0.5 0.5 0.5)) "AlwaysSpawn" "OverrideRootScale" null null))
  (`/Game/GameComponents/BP_PlayerTrip.CreatePawn` _returnvalue 2 Name (`BlueprintMapLibrary.Map_Find` (`self.Materials`) 2) true)
  (`KismetArrayLibrary.Array_Add` (`self.ArrayPlayersSpawn`) _returnvalue))

(event `Start Game`
  (bind _asbp_player_controller_trip (cast `/Game/GameComponents/BP_PlayerControllerTrip` (`GameplayStatics.GetPlayerController` 0)))
  (`/Game/GameComponents/BP_PlayerControllerTrip.Event Set Player` _asbp_player_controller_trip (`self.ArrayPlayersSpawn`)))

(event `Event Create Pawn 3`
  (params (Name :type Text))
  (bind _returnvalue (`|SpawnActorFromClass` "/Game/GameComponents/BP_PlayerTrip.BP_PlayerTrip_C" (`KismetMathLibrary.MakeTransform` (`SceneComponent.K2_GetComponentLocation` (`self.PlayerStay2`)) (struct) (0.5 0.5 0.5)) "AlwaysSpawn" "OverrideRootScale" null null))
  (`/Game/GameComponents/BP_PlayerTrip.CreatePawn` _returnvalue 3 Name (`BlueprintMapLibrary.Map_Find` (`self.Materials`) 3) true)
  (`KismetArrayLibrary.Array_Add` (`self.ArrayPlayersSpawn`) _returnvalue))

(event `Event Create Pawn 4`
  (params (Name :type Text))
  (bind _returnvalue (`|SpawnActorFromClass` "/Game/GameComponents/BP_PlayerTrip.BP_PlayerTrip_C" (`KismetMathLibrary.MakeTransform` (`SceneComponent.K2_GetComponentLocation` (`self.PlayerStay3`)) (struct) (0.5 0.5 0.5)) "AlwaysSpawn" "OverrideRootScale" null null))
  (`/Game/GameComponents/BP_PlayerTrip.CreatePawn` _returnvalue 4 Name (`BlueprintMapLibrary.Map_Find` (`self.Materials`) 4) true)
  (`KismetArrayLibrary.Array_Add` (`self.ArrayPlayersSpawn`) _returnvalue))

(fn `UserConstructionScript`
  (`parent.UserConstructionScript`))