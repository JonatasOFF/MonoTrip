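; BP_LocalSorter is a chance-card space in a board game, drawing one of four random cards for the player passed to CallLocal.
; Each card shows its widget, then grants an Amazonia pass, moves the player toward the airport, exchanges money among players, or enables house destruction.
; Destruction flags other players' properties, with bots calling DestroyHouse on random picks, and skips to the next round when no properties exist.
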(event `self.Call Local`
  (params (PlayerTrip :type "/Game/GameComponents/BP_PlayerTrip Object Reference"))
  (bind _player (`self.Player`))
  (bind _indexnow (`/Game/GameComponents/BP_PlayerTrip.IndexNow` _player))
  (bind _players (`/Game/GameComponents/BP_PlayerControllerTrip.Players` (`self.PlayerController`)))
  (bind _players_2 (`/Game/GameComponents/BP_PlayerControllerTrip.Players` (`self.PlayerController`)))
  (bind _returnvalue (- 24 _indexnow))
  (bind _output_get (set `self.Player` PlayerTrip))
  (bind _asbp_player_controller_trip (cast `/Game/GameComponents/BP_PlayerControllerTrip` (`GameplayStatics.GetPlayerController` 0)))
  (set `self.PlayerController` _asbp_player_controller_trip)
  (switch `int` (`KismetMathLibrary.RandomIntegerInRange` 1 4)
    (:`1`
      (bind _returnvalue_2 (`|CreateWidget` "/Game/Widgets/WidgetSortier/BP_CartaSairAmazonia.BP_CartaSairAmazonia_C"))
      (`UserWidget.AddToViewport` _returnvalue_2 0)
      (set `/Game/GameComponents/BP_PlayerTrip.isHavePassToAmazonia` true _output_get))
    (:`2`
      (bind _returnvalue_3 (`|CreateWidget` "/Game/Widgets/WidgetSortier/BP_AeroportoNow.BP_AeroportoNow_C"))
      (`UserWidget.AddToViewport` _returnvalue_3 0)
      (if (> _indexnow 24)
        (`/Game/GameComponents/BP_PlayerControllerTrip.Movement Player` (`self.PlayerController`) _player 28 28)
        (else
          (`/Game/GameComponents/BP_PlayerControllerTrip.Movement Player` (`self.PlayerController`) _player _returnvalue _returnvalue))))
    (:`3`
      (bind _returnvalue_4 (`|CreateWidget` "/Game/Widgets/WidgetSortier/BP_Pega25Cada.BP_Pega25Cada_C"))
      (`UserWidget.AddToViewport` _returnvalue_4 0)
      (for _array_element _players
        (`/Game/GameComponents/BP_PlayerTrip.SetNewMoney` _array_element 50000 false true))
      (`/Game/GameComponents/BP_PlayerTrip.SetNewMoney` (`self.Player`) (- (* (`KismetArrayLibrary.Array_Length` _players) -50000) 50000) false false))
    (:`4`
      (bind _returnvalue_5 (`|CreateWidget` "/Game/Widgets/WidgetSortier/BP_DestruirCasa.BP_DestruirCasa_C"))
      (`UserWidget.AddToViewport` _returnvalue_5 0)
      (for _array_element_2 _players_2
        (if (not (== _array_element_2 (`self.Player`)))
          (bind _localshave (`/Game/GameComponents/BP_PlayerTrip.LocalsHave` _array_element_2))
          (bind _returnvalue_6 (`KismetArrayLibrary.Array_Length` _localshave))
          (if (!= _returnvalue_6 0)
            (for _array_element_3 _localshave
              (set `self.isGetHouse` true)
              (bind _asbp_local_casa (cast `/Game/Lugares/BP_LocalCasa` _array_element_3))
              (set `/Game/Lugares/BP_LocalCasa.isDestroyHouse` true _asbp_local_casa))
            (if (`/Game/GameComponents/BP_PlayerTrip.isBot` (`self.Player`))
              (bind _localshave_2 (`/Game/GameComponents/BP_PlayerTrip.LocalsHave` (`|GetArrayItem` _players_2 (`KismetMathLibrary.RandomInteger` _returnvalue_6))))
              (bind _asbp_local_casa_2 (cast `/Game/Lugares/BP_LocalCasa` (`|GetArrayItem` _localshave_2 (`KismetMathLibrary.RandomInteger` (`KismetArrayLibrary.Array_Length` _localshave_2)))))
              (`/Game/Lugares/BP_LocalCasa.DestroyHouse` _asbp_local_casa_2)))))
      (if (not (`self.isGetHouse`))
        (`/Game/FunctionsBot/BP_FunctionFromBot.Go Next Round`)))))

(fn `UserConstructionScript`
  (`parent.UserConstructionScript`))