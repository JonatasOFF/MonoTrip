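; Blueprint function that hands the turn to the current player in the Trip dice board game.
; It looks up the player at IndexGo in BP_PlayerControllerTrip's Players list.
; Players flagged IsAeroporto are passed to BP_GameModeTrip's airport event.
; Otherwise the first BP_PlayDice widget rolls automatically for bots or shows the Go button for humans.
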(fn `Go Next Round`
  (bind _asbp_player_controller_trip (cast `/Game/GameComponents/BP_PlayerControllerTrip` (`GameplayStatics.GetPlayerController` null)))
  (bind _foundwidgets (`WidgetBlueprintLibrary.GetAllWidgetsOfClass` null "/Game/Widgets/BP_PlayDice.BP_PlayDice_C"))
  (bind _output (`|GetArrayItem` (`/Game/GameComponents/BP_PlayerControllerTrip.Players` _asbp_player_controller_trip) (`/Game/GameComponents/BP_PlayerControllerTrip.IndexGo` _asbp_player_controller_trip)))
  (if (`/Game/GameComponents/BP_PlayerTrip.isAeroporto` _output)
    (bind _asbp_game_mode_trip (cast `/Game/GameComponents/BP_GameModeTrip` (`GameplayStatics.GetGameMode` null)))
    (`/Game/GameComponents/BP_GameModeTrip.Event Set Aeroporto` _asbp_game_mode_trip _output)
    (elif (`/Game/GameComponents/BP_PlayerTrip.isBot` _output)
      (bind _output_2 (`|GetArrayItem` _foundwidgets))
      (`/Game/Widgets/BP_PlayDice.Event Click Go` _output_2)
      (else
        (`/Game/Widgets/BP_PlayDice.ShowClickGo` _output_2)))))